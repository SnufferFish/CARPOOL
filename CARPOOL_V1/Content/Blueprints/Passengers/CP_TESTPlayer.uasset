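; CP_TESTPlayer is a test player actor for the passenger and vehicle systems.
; On BeginPlay it shows TestHUD with the mouse cursor, then spawns a TEST_VEH1, stores it as CPPlayerVehicle and attaches it to itself.
; Clicking the avatar prints each vehicle passenger's name and job from class defaults.
; Releasing the click prints the player's name, job and age from CP_GameInstance to test that data.
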(event `self.ReceiveBeginPlay`
  (bind _returnvalue (`GameplayStatics.GetPlayerController` 0))
  (bind _returnvalue_2 (`|CreateWidget` "/Game/Blueprints/HUD/TestHUD.TestHUD_C" _returnvalue))
  (`UserWidget.AddToViewport` _returnvalue_2 0)
  (set `PlayerController.bShowMouseCursor` true _returnvalue)
  ;[1 1 1] Set Reference to Vehicle
  (bind _returnvalue_3 (`|SpawnActorFromClass` "/Game/Blueprints/Vehicles/TEST_VEH1.TEST_VEH1_C" (`KismetMathLibrary.MakeTransform` (165.0 0.0 160.0)) "Undefined" "OverrideRootScale"))
  (set `self.CP_PlayerVehicle` _returnvalue_3)
  ;[1 1 1] attaching vehicle actor to cp actor for some reason
  (`self.K2_AttachToActor` _returnvalue_3 self "None" "KeepRelative" "KeepRelative" "KeepRelative" true))

(event `self.PLAYER_Avatar.OnClicked`
  (params (TouchedComponent :type "PrimitiveComponent Object Reference") (ButtonPressed :type "Key Structure" :default "AnyKey"))
  (for _array_element (`CP_VEHICLE.aPassengersInVehicle` (`self.CP_PlayerVehicle`))
    (bind (_passenger_name _passenger_age _is_driver _passenger_job) (defaults `/Game/Blueprints/Passengers/CP_TESTPlayer` _array_element))
    (`KismetSystemLibrary.PrintString` (`KismetStringLibrary.Concat_StrStr` (`|GetEnumeratorNameAsString` _passenger_name) " " (`|GetEnumeratorNameAsString` _passenger_job)))))

(event `self.PLAYER_Avatar.OnReleased`
  (params (TouchedComponent :type "PrimitiveComponent Object Reference") (ButtonReleased :type "Key Structure" :default "AnyKey"))
  (bind _ascp_game_instance (cast `CP_GameInstance` (`GameplayStatics.GetGameInstance`)))
  ;[1 1 1] Game Instance test
  (set `self.PlayerNameFromHUD` (`CP_GameInstance.PlayerNameFromHUD` _ascp_game_instance))
  (set `self.PLAYER_Age` (`CP_GameInstance.PassengerAge` _ascp_game_instance))
  (set `self.PLAYER_Job` (`CP_GameInstance.SelectedJob` _ascp_game_instance))
  (`KismetSystemLibrary.PrintString` (`KismetStringLibrary.Concat_StrStr` (`KismetTextLibrary.Conv_TextToString` (`self.PlayerNameFromHUD`)) " " (`|GetEnumeratorNameAsString` (`self.PLAYER_Job`)) " " (`KismetStringLibrary.Conv_IntToString` (`self.PLAYER_Age`)))))

(fn `UserConstructionScript`)