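; TestPassenger is a test passenger actor with a clickable avatar that reports which passenger it is.
; Its construction script calls InitiatePassenger, whose body is defined outside this graph.
; On BeginPlay it adds a TestHUD widget to the viewport and shows player 0's mouse cursor.
; Clicking PASSENGER_Avatar prints the PASSENGERName enum value as a debug string.
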(event `self.ReceiveBeginPlay`
  (bind _returnvalue (`GameplayStatics.GetPlayerController` 0))
  (bind _returnvalue_2 (`|CreateWidget` "/Game/Blueprints/HUD/TestHUD.TestHUD_C" _returnvalue))
  (bind _output_get (set `self.NewVar_0` _returnvalue_2))
  (`UserWidget.AddToViewport` _output_get 0)
  (set `PlayerController.bShowMouseCursor` true _returnvalue))

(event `self.PASSENGER_Avatar.OnClicked`
  (params (TouchedComponent :type "PrimitiveComponent Object Reference") (ButtonPressed :type "Key Structure" :default "AnyKey"))
  (`KismetSystemLibrary.PrintString` (`|GetEnumeratorNameAsString` (`self.PASSENGER_Name`))))

(fn `UserConstructionScript`
  (`self.InitiatePassenger`))